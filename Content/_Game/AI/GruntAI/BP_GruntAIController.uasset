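; AI controller for the grunt enemy that starts its behavior tree and feeds it player detection.
; On possess it runs BT_GruntEnemy.
; When AI perception successfully senses an actor tagged Player, it sets the Sight flag and stores that actor as EnemyActor on the blackboard.
; Nothing here clears those keys when the player is no longer sensed.
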(event OnTargetPerceptionUpdated(AIPerception)
  (params (Actor :type Actor%20Object%20Reference) (Stimulus :type AI%20Stimulus%20Structure))
  (bind _blackboard (Variables|Default|GetBlackboard))
  (if (and (Actor|ActorHasTag Actor "Player") (.bSuccessfullySensed (Utilities|Struct|BreakAIStimulus Stimulus)))
    (AI|Components|Blackboard|SetValueasBool _blackboard (Variables|Default|GetSight) true)
    (AI|Components|Blackboard|SetValueasObject _blackboard (Variables|Default|GetEnemyActor) Actor)))

(event EventBeginPlay)

(event EventTick
  (params (DeltaSeconds :type Float%20%28single-precision%29)))

(event EventPossess
  (params (PossessedPawn :type Pawn%20Object%20Reference))
  (AI|RunBehaviorTree "/Game/_Game/AI/GruntAI/BT_GruntEnemy.BT_GruntEnemy"))

(fn ConstructionScript)